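; BP_MainObject is a collectible pickup that counts toward winning the game.
; A timeline started on BeginPlay animates the sprite's relative location.
; When the hero overlaps the sphere, the pickup increments the hero's PickUps count and destroys itself, showing the win screen and pausing the game once the target count is reached.
; A custom event toggles visibility of the sprite, sphere and glow together.
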(event OnComponentBeginOverlap(Sphere)
  (params (OverlappedComponent :type Primitive%20Component%20Object%20Reference) (OtherActor :type Actor%20Object%20Reference) (OtherComp :type Primitive%20Component%20Object%20Reference) (OtherBodyIndex :type Integer) (bFromSweep :type Boolean) (SweepResult :type Hit%20Result%20Structure%20%28by%20ref%29))
  (bind _asbp_hero_character (Utilities|Casting|CastToBP_HeroCharacter OtherActor))
  (Variables|/Game/Blueprints/Hero/BP_HeroCharacter.BP_HeroCharacter_C|SetPickUps _asbp_hero_character (+ (Variables|/Game/Blueprints/Hero/BP_HeroCharacter.BP_HeroCharacter_C|GetPickUps _asbp_hero_character) 1))
  (Actor|DestroyActor)
  (if (>= (Variables|/Game/Blueprints/Hero/BP_HeroCharacter.BP_HeroCharacter_C|GetPickUps _asbp_hero_character) 5)
    (bind _returnvalue (UserInterface|CreateWidget "/Game/UI/QuestAndStart/W_WinScreen.W_WinScreen_C"))
    (UserInterface|Viewport|AddtoViewport _returnvalue 0)
    (Game|SetGamePaused true)))

(event Custom|ChangeComponentVisibility
  (params (Visible? :type Boolean))
  (Rendering|SetVisibility (Variables|Default|GetPaper%20Sprite) Visible? false))

(event EventBeginPlay
  (bind _asbp_hero_character (Utilities|Casting|CastToBP_HeroCharacter (Game|GetPlayerCharacter 0)))
  (Variables|Default|SetBP_HeroCharacter _asbp_hero_character)
  (bind _newtrack_0 (Timeline|Timeline Play)
    (:Update
      (Transformation|SetRelativeLocation (Variables|Default|GetPaper%20Sprite) _newtrack_0 false false))))

(fn ConstructionScript)