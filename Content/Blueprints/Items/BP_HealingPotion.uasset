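; BP_HealingPotion is a health pickup with a Paper2D sprite animated by a timeline from BeginPlay.
; Any Sphere overlap while the cached player hero is below max health triggers a one-time heal, without checking the overlapping actor.
; It adds PotionHeal below a hardcoded health threshold, otherwise fills to max, then reports the health ratio to the hero.
; A MoveUp timeline then moves the sprite, and a short delay precedes destruction.
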(event OnComponentBeginOverlap(Sphere)
  (params (OverlappedComponent :type Primitive%20Component%20Object%20Reference) (OtherActor :type Actor%20Object%20Reference) (OtherComp :type Primitive%20Component%20Object%20Reference) (OtherBodyIndex :type Integer) (bFromSweep :type Boolean) (SweepResult :type Hit%20Result%20Structure%20%28by%20ref%29))
  (bind _bp_herocharacter (Variables|Default|GetBP_HeroCharacter))
  (bind _bp_herocharacter_2 (Variables|Default|GetBP_HeroCharacter))
  (bind _bp_herocharacter_3 (Variables|Default|GetBP_HeroCharacter))
  (bind _bp_herocharacter_4 (Variables|Default|GetBP_HeroCharacter))
  (if (< (Variables|/Game/Blueprints/Hero/BP_HeroCharacter.BP_HeroCharacter_C|GetHealth _bp_herocharacter_2) (Variables|/Game/Blueprints/Hero/BP_HeroCharacter.BP_HeroCharacter_C|GetMaxHealth _bp_herocharacter_2))
    (Utilities|FlowControl|DoOnce false
      (:Completed
        (if (< (Variables|/Game/Blueprints/Hero/BP_HeroCharacter.BP_HeroCharacter_C|GetHealth (Variables|Default|GetBP_HeroCharacter)) 5e+01)
          (Variables|/Game/Blueprints/Hero/BP_HeroCharacter.BP_HeroCharacter_C|SetHealth _bp_herocharacter (+ (Variables|/Game/Blueprints/Hero/BP_HeroCharacter.BP_HeroCharacter_C|GetHealth _bp_herocharacter) (Variables|Default|GetPotionHeal)))
          (else
            (Variables|/Game/Blueprints/Hero/BP_HeroCharacter.BP_HeroCharacter_C|SetHealth _bp_herocharacter_4 (Variables|/Game/Blueprints/Hero/BP_HeroCharacter.BP_HeroCharacter_C|GetMaxHealth _bp_herocharacter_4))))
        (Default|CallChangingHealth _bp_herocharacter (/ (Variables|/Game/Blueprints/Hero/BP_HeroCharacter.BP_HeroCharacter_C|GetHealth _bp_herocharacter_3) (Variables|/Game/Blueprints/Hero/BP_HeroCharacter.BP_HeroCharacter_C|GetMaxHealth _bp_herocharacter_3)))
        (bind _newtrack_0 (Timeline|MoveUp Play)
          (:Update
            (Transformation|SetRelativeLocation (Variables|Default|GetPaperSprite) _newtrack_0 false false)
            (Utilities|FlowControl|Delay 0.4)
            (Actor|DestroyActor)))))))

(event EventBeginPlay
  (bind _asbp_hero_character (Utilities|Casting|CastToBP_HeroCharacter (Game|GetPlayerCharacter 0)))
  (Variables|Default|SetBP_HeroCharacter _asbp_hero_character)
  (bind _newtrack_0 (Timeline|Moving Play)
    (:Update
      (Transformation|SetRelativeLocation (Variables|Default|GetPaperSprite) _newtrack_0 false false))))

(event Collision|EventActorBeginOverlap
  (params (OtherActor :type Actor%20Object%20Reference)))

(event EventTick
  (params (DeltaSeconds :type Float%20%28single-precision%29)))

(fn ConstructionScript)