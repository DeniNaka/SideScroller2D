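; BP_Enemy is a side-scrolling enemy character that patrols along X, hurts the hero on contact and can be killed.
; Despite its name, Follow runs on Tick as a back-and-forth patrol, counting steps toward S, then flipping its sign and the sprite.
; Damage knocks it away from the hero and briefly locks movement; death grants the hero Mana and delays destruction.
; BoxHit overlap damages the hero, passes it the enemy's X position and pauses the patrol.
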(event OnComponentBeginOverlap(BoxHit)
  (params (OverlappedComponent :type Primitive%20Component%20Object%20Reference) (OtherActor :type Actor%20Object%20Reference) (OtherComp :type Primitive%20Component%20Object%20Reference) (OtherBodyIndex :type Integer) (bFromSweep :type Boolean) (SweepResult :type Hit%20Result%20Structure%20%28by%20ref%29))
  (bind _returnvalue (Components|GetOwner))
  (Utilities|IsValid _returnvalue
    (:Is%20Valid
      (if (not (== OtherActor _returnvalue))
        (bind _asbp_hero_character (Utilities|Casting|CastToBP_HeroCharacter OtherActor))
        (Game|Damage|ApplyDamage _asbp_hero_character (Variables|Default|GetDamageToCharacter) 0 0)
        (Variables|/Game/Blueprints/Hero/BP_HeroCharacter.BP_HeroCharacter_C|SetEnemyPositionX (Variables|Default|GetBP%20Hero%20Character) (.x (Transformation|GetWorldLocation (Variables|Default|GetSprite))))
        (Variables|Default|SetisMovementLocked? true)
        (Utilities|FlowControl|Delay 2.0)
        (Variables|Default|SetisMovementLocked? false)))))

(event Custom|Follow
  (if (not (Variables|Default|GetisMovementLocked?))
    (Math|Float|CompareFloat (Variables|Default|GetS1) (Variables|Default|GetS)
      (:>
        (Pawn|Input|AddMovementInput "-1.000000,0.000000,0.000000" 1.0 false)
        (Variables|Default|SetS1 (- (Variables|Default|GetS1) 1.0)))
      (:==
        (if (> (Variables|Default|GetS) 0.0)
          (Variables|Default|SetS (* (Variables|Default|GetS) -1.0))
          (Variables|Default|SetS1 0.0)
          (Transformation|SetRelativeRotation (Variables|Default|GetSprite) "0.000000,180.000000,0.000000" false false)
          (else
            (Variables|Default|SetS (* (Variables|Default|GetS) -1.0))
            (Variables|Default|SetS1 0.0)
            (Transformation|SetRelativeRotation (Variables|Default|GetSprite) "0, 0, 0" false false))))
      (:<
        (Pawn|Input|AddMovementInput "1.000000,0.000000,0.000000" 1.0 false)
        (Variables|Default|SetS1 (+ (Variables|Default|GetS1) 1.0))))))

(event EventBeginPlay
  (bind _asbp_hero_character (Utilities|Casting|CastToBP_HeroCharacter (Game|GetPlayerCharacter 0)))
  (Variables|Default|SetBP%20Hero%20Character _asbp_hero_character))

(event Game|Damage|EventAnyDamage
  (params (Damage :type Float%20%28single-precision%29) (DamageType :type Damage%20Type%20Object%20Reference) (InstigatedBy :type Controller%20Object%20Reference) (DamageCauser :type Actor%20Object%20Reference))
  (bind _bp_hero_character (Variables|Default|GetBP%20Hero%20Character))
  ;[0.1125 0.1125 0.1125] Launch Enemy and Death
  (if (not (Variables|Default|GetisDeath?))
    (Math|Float|CompareFloat (.x (Transformation|GetWorldLocation (Variables|/Script/Paper2D.PaperCharacter|GetSprite (Variables|Default|GetBP%20Hero%20Character)))) (.x (Transformation|GetWorldLocation (Variables|Default|GetSprite)))
      (:>
        (Character|LaunchCharacter "-500.000000,0.000000,200.000000" true true))
      (:<
        (Character|LaunchCharacter "500.000000,0.000000,200.000000" true true)))
    (Variables|Default|SetHealth (- (Variables|Default|GetHealth) Damage))
    (Variables|Default|SetisTakingDamage? true)
    (Development|PrintString (Utilities|String|Append "Remain Health: " (Utilities|String|ToString(Float) (Variables|Default|GetHealth))))
    (if (> (Variables|Default|GetHealth) 0.0)
      (Variables|Default|SetisMovementLocked? true)
      (Utilities|FlowControl|Delay 0.65)
      (Variables|Default|SetisMovementLocked? false)
      (Variables|Default|SetisTakingDamage? false)
      (else
        (Variables|Default|SetDamageToCharacter 0.0)
        (Variables|/Game/Blueprints/Hero/BP_HeroCharacter.BP_HeroCharacter_C|SetMana _bp_hero_character (+ (Variables|/Game/Blueprints/Hero/BP_HeroCharacter.BP_HeroCharacter_C|GetMana _bp_hero_character) 3e+01))
        (Variables|Default|SetisDeath? true)
        (Utilities|FlowControl|Delay 0.1)
        (Variables|Default|SetisMovementLocked? true)
        (Utilities|FlowControl|Delay 1.3)
        (Actor|DestroyActor)))
    (else
      (Variables|Default|SetisMovementLocked? true))))

(event EventTick
  (params (DeltaSeconds :type Float%20%28single-precision%29))
  (CallFunction|Follow))

(fn ConstructionScript)